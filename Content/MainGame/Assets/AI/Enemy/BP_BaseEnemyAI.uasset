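; Base melee enemy AI that chases and attacks the Dangle_BP player, with a proximity-shown health bar.
; Sight, detector overlap or TakeDamage triggers AIMoveTo and a smash montage, whose notify applies damage if the player is inside AttackBox.
; Death ragdolls then destroys it; player death disables sensing, while OnReset returns it to its stored spawn and re-enables sensing.
; Tick tracks movement state and interpolates walk speed.
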(event OnSeePawn(PawnSensing)
  (params (Pawn :type Pawn%20Object%20Reference))
  ;[1 1 1] AttackPlayer
  (bind _asdangle_bp (Utilities|Casting|CastToDangle_BP Pawn))
  (Variables|Default|SetThirdPersonCharacter _asdangle_bp)
  (if (not (Variables|Default|Getis%20Attacking))
    (AI|AIMoveTo self "0, 0, 0" (Pawn|GetControlledPawn (Game|GetPlayerController 0)) 1.0 false
      (:OnSuccess
        (Variables|Default|Setis%20Attacking true)
        (Animation|Montage|PlayMontage (Variables|Character|GetMesh) "/Game/MainGame/Assets/Dangle/Meshes/Dangle/Animations/Fighting/AISmashIncplace.AISmashIncplace" 2.0
          (:OnCompleted
            (Variables|Default|Setis%20Attacking false))
          (:OnNotifyBegin
            (if (Variables|Default|GetInRange)
              (Game|Damage|ApplyDamage (Variables|Default|GetThirdPersonCharacter) (Math|Conversions|ToFloat(Integer) (Variables|Default|GetAttackDamage)) 0 0))))))))

(event OnComponentBeginOverlap(AttackBox)
  (params (OverlappedComponent :type Primitive%20Component%20Object%20Reference) (OtherActor :type Actor%20Object%20Reference) (OtherComp :type Primitive%20Component%20Object%20Reference) (OtherBodyIndex :type Integer) (bFromSweep :type Boolean) (SweepResult :type Hit%20Result%20Structure%20%28by%20ref%29))
  ;[1 1 1] Detect If Player In Range
  (bind _asdangle_bp (Utilities|Casting|CastToDangle_BP (Game|GetPlayerCharacter 0)))
  (if (== OtherComp (Variables|/Script/Engine.Character|GetCapsuleComponent _asdangle_bp))
    (Variables|Default|SetInRange true)))

(event OnComponentEndOverlap(AttackBox)
  (params (OverlappedComponent :type Primitive%20Component%20Object%20Reference) (OtherActor :type Actor%20Object%20Reference) (OtherComp :type Primitive%20Component%20Object%20Reference) (OtherBodyIndex :type Integer))
  ;[1 1 1] Detect If Player In Range
  (bind _asdangle_bp (Utilities|Casting|CastToDangle_BP (Game|GetPlayerCharacter 0)))
  (if (== OtherComp (Variables|/Script/Engine.Character|GetCapsuleComponent _asdangle_bp))
    (Variables|Default|SetInRange false)))

(event OnComponentBeginOverlap(HealthVisability)
  (params (OverlappedComponent :type Primitive%20Component%20Object%20Reference) (OtherActor :type Actor%20Object%20Reference) (OtherComp :type Primitive%20Component%20Object%20Reference) (OtherBodyIndex :type Integer) (bFromSweep :type Boolean) (SweepResult :type Hit%20Result%20Structure%20%28by%20ref%29))
  ;[1 1 1] HealthBox Visability
  (if (not (Variables|Default|GetisDead))
    (Utilities|Casting|CastToDangle_BP OtherActor)
    (Rendering|SetVisibility (Variables|Default|GetEnemyHealthUI) true true)))

(event OnComponentEndOverlap(HealthVisability)
  (params (OverlappedComponent :type Primitive%20Component%20Object%20Reference) (OtherActor :type Actor%20Object%20Reference) (OtherComp :type Primitive%20Component%20Object%20Reference) (OtherBodyIndex :type Integer))
  ;[1 1 1] HealthBox Visability
  (if (not (Variables|Default|GetisDead))
    (Utilities|Casting|CastToDangle_BP OtherActor)
    (Rendering|SetVisibility (Variables|Default|GetEnemyHealthUI) false true)))

(event OnComponentBeginOverlap(PlayerDetector)
  (params (OverlappedComponent :type Primitive%20Component%20Object%20Reference) (OtherActor :type Actor%20Object%20Reference) (OtherComp :type Primitive%20Component%20Object%20Reference) (OtherBodyIndex :type Integer) (bFromSweep :type Boolean) (SweepResult :type Hit%20Result%20Structure%20%28by%20ref%29))
  ;[1 1 1] AttackPlayer
  (bind _asdangle_bp (Utilities|Casting|CastToDangle_BP OtherActor))
  (Variables|Default|SetPlayerInSights true)
  (Transformation|SetActorRotation (Math|Rotator|MakeRotator (.roll (Math|Rotator|FindLookatRotation (Transformation|GetActorLocation) (Transformation|GetActorLocation _asdangle_bp))) 0.0 (.yaw (Math|Rotator|FindLookatRotation (Transformation|GetActorLocation) (Transformation|GetActorLocation _asdangle_bp)))))
  (CallFunction|GotHit (Game|GetPlayerCharacter 0)))

(event OnComponentEndOverlap(PlayerDetector)
  (params (OverlappedComponent :type Primitive%20Component%20Object%20Reference) (OtherActor :type Actor%20Object%20Reference) (OtherComp :type Primitive%20Component%20Object%20Reference) (OtherBodyIndex :type Integer))
  ;[1 1 1] AttackPlayer
  (Utilities|Casting|CastToDangle_BP OtherActor)
  (Variables|Default|SetPlayerInSights false))

(event Custom|CheckHealth
  (params (Health :type Float%20%28single-precision%29))
  ;[1 1 1] AIDies
  (if (not (>= Health 1.0))
    (Utilities|FlowControl|DoOnce false
      (:Completed
        (Pawn|Components|CharacterMovement|DisableMovement (Variables|Character|GetCharacterMovement))
        (Audio|PlaySound2D "/Game/Audio/Dangle_death_sound.Dangle_death_sound" 0.2 0.76 0.65 0 0)
        (Class|PawnSensingComponent|SetSensingUpdatesEnabled (Variables|Default|GetPawnSensing) false)
        (Collision|SetCollisionEnabled (Variables|Collision|GetCapsuleComponent) "NoCollision")
        (Physics|SetSimulatePhysics (Variables|Character|GetMesh) true)
        (Rendering|SetVisibility (Variables|Default|GetEnemyHealthUI) false false)
        (Variables|Default|SetisDead true)
        (Utilities|FlowControl|Delay 1e+01)
        (Actor|DestroyActor)))))

(event Custom|ResetAI
  ;[1 1 1] Reset it player Dies
  (Development|PrintString "resetting AI")
  (Class|PawnSensingComponent|SetSensingUpdatesEnabled (Variables|Default|GetPawnSensing) false))

(event Custom|GotHit
  (params (Pawn :type Pawn%20Object%20Reference))
  ;[1 1 1] AttackPlayer
  (bind _asdangle_bp (Utilities|Casting|CastToDangle_BP Pawn))
  (Variables|Default|SetThirdPersonCharacter _asdangle_bp)
  (if (not (Variables|Default|Getis%20Attacking))
    (AI|AIMoveTo self "0, 0, 0" (Pawn|GetControlledPawn (Game|GetPlayerController 0)) 1.0 false
      (:OnSuccess
        (Variables|Default|Setis%20Attacking true)
        (Animation|Montage|PlayMontage (Variables|Character|GetMesh) "/Game/MainGame/Assets/Dangle/Meshes/Dangle/Animations/Fighting/AISmashIncplace.AISmashIncplace" 2.0
          (:OnCompleted
            (Variables|Default|Setis%20Attacking false))
          (:OnNotifyBegin
            (if (Variables|Default|GetInRange)
              (Game|Damage|ApplyDamage (Variables|Default|GetThirdPersonCharacter) (Math|Conversions|ToFloat(Integer) (Variables|Default|GetAttackDamage)) 0 0))))))))

(event EventBeginPlay
  (Utilities|FlowControl|Sequence
    (:then_0
      ;[1 1 1] Save AI Starting Location
      (if (not (Variables|Default|GetHasLocationStored))
        (Variables|Default|SetActorSpawnLocation (Transformation|GetActorLocation))
        (Variables|Default|SetActorSpawnRotation (Transformation|GetActorRotation))
        (Variables|Default|SetHasLocationStored true)))
    (:then_1
      ;[1 1 1] Reset it player Dies
      (bind _asdangle_bp (Utilities|Casting|CastToDangle_BP (Game|GetPlayerCharacter 0)))
      (EventDispatchers|AssignPlayerDied _asdangle_bp (delegate Custom|ResetAI)))
    (:then_2
      ;;[1 0.99 0.1639] Set Visability of Health Bar
      (Utilities|FlowControl|Delay 0.2)
      (Rendering|SetVisibility (Variables|Default|GetEnemyHealthUI) false true))
    (:then_3
      ;;[1 0 0.08657] Define Enemy UI
      (bind _asenemy_health_ui (Utilities|Casting|CastToEnemyHealthUI (UserInterface|GetUserWidgetObject (Variables|Default|GetEnemyHealthUI))))
      (Variables|/Game/MainGame/Assets/AI/UI/EnemyHealthUI.EnemyHealthUI_C|SetEnemy1 _asenemy_health_ui self))
    (:then_4
      ;;[0.08708 1 0] Store EnemyVar
      (bind _asstore_vars_1 (Utilities|Casting|CastToStoreVars_1 (Game|GetGameInstance)))
      (Variables|/Game/MainGame/StoreVars_1.StoreVars_1_C|SetEnemy _asstore_vars_1 self))))

(event Game|Damage|EventAnyDamage
  (params (Damage :type Float%20%28single-precision%29) (DamageType :type Damage%20Type%20Object%20Reference) (InstigatedBy :type Controller%20Object%20Reference) (DamageCauser :type Actor%20Object%20Reference))
  ;[1 1 1] AIDies
  (Variables|Default|SetPlayerHealth (- (Variables|Default|GetPlayerHealth) Damage))
  (if (not (>= (stale Custom|CheckHealth Health) 1.0))
    (Utilities|FlowControl|DoOnce false
      (:Completed
        (Pawn|Components|CharacterMovement|DisableMovement (Variables|Character|GetCharacterMovement))
        (Audio|PlaySound2D "/Game/Audio/Dangle_death_sound.Dangle_death_sound" 0.2 0.76 0.65 0 0)
        (Class|PawnSensingComponent|SetSensingUpdatesEnabled (Variables|Default|GetPawnSensing) false)
        (Collision|SetCollisionEnabled (Variables|Collision|GetCapsuleComponent) "NoCollision")
        (Physics|SetSimulatePhysics (Variables|Character|GetMesh) true)
        (Rendering|SetVisibility (Variables|Default|GetEnemyHealthUI) false false)
        (Variables|Default|SetisDead true)
        (Utilities|FlowControl|Delay 1e+01)
        (Actor|DestroyActor)))))

(event EventOnReset
  (bind _actorspawnlocation (Variables|Default|GetActorSpawnLocation))
  ;[1 1 1] OnResetGame
  (Development|PrintString "ResetAI Game")
  (Transformation|Teleport _actorspawnlocation (Variables|Default|GetActorSpawnRotation))
  (AI|AIMoveTo self _actorspawnlocation 0 5.0 false
    (:then
      (Class|PawnSensingComponent|SetSensingUpdatesEnabled (Variables|Default|GetPawnSensing) true))))

(event EventTick
  (params (DeltaSeconds :type Float%20%28single-precision%29))
  (bind _returnvalue (Transformation|GetVelocity))
  (Variables|Default|SetDelta DeltaSeconds)
  ;[1 1 1] Gets the character's rate of rotation. Used to lean the character while turning.
  (Variables|Default|SetCurrentRotationRate (Math|Float|MapRangeClamped (.Z (Math|Vector|BreakVector (Physics|GetPhysicsAngularVelocityinDegrees (Variables|Collision|GetCapsuleComponent) "None"))) -3.6e+02 3.6e+02 -1.0 1.0))
  ;[1 1 1] Determine if character is moving.
  (Variables|Default|SetIsMoving (Math|Vector|NotEqual(Vector) (Transformation|GetComponentVelocity (Variables|Collision|GetCapsuleComponent)) "0, 0, 0" 0.0001))
  ;[1 1 1] Determine if character is currently accelerating.
  (bind _output_get (Variables|Default|SetIsAccelerating (> (Math|Vector|VectorLength (Pawn|Components|CharacterMovement|GetCurrentAcceleration (Variables|Character|GetCharacterMovement))) 0.0)))
  ;[1 1 1] If character is coming to a stop, record its last known speed so that we know how fast it was moving before slowing down. This value isn't changed again unless the player starts moving, then stops again.
  (if _output_get
    (goto _label Reset%20In)
    (else
      (Utilities|FlowControl|Sequence
        (:then_0
          (|DoOnceMultiInput :!label _label
            (:A%20Out
              (Variables|Default|SetSpeedWhenStopping (Variables|Default|GetCurrentSpeed)))
            (:Reset%20Out
              ;[1 1 1] Record the character's current speed.
              (Variables|Default|SetCurrentSpeed (Math|Vector|VectorLength _returnvalue) :!label _label_2)
              ;[1 1 1] Record the character's current lateral speed.
              (Variables|Default|SetLateralSpeed (Math|Vector|VectorLengthXY _returnvalue))
              ;[1 1 1] Adjust max movement speed for walking/jogging/running.
              (Variables|/Script/Engine.CharacterMovementComponent|SetMaxWalkSpeed (Variables|Character|GetCharacterMovement) (Math|Interpolation|FInterpTo (Variables|/Script/Engine.CharacterMovementComponent|GetMaxWalkSpeed (Variables|Character|GetCharacterMovement)) (Variables|Default|GetMaxSpeedTarget) (Variables|Default|GetDelta) 4.0)))))
        (:then_1
          (goto _label_2))))))

(fn ConstructionScript)

(fn TakeDamage
  (params (Damage :type Float%20%28single-precision%29))
  (Utilities|FlowControl|Sequence
    (:then_0
      (bind _output_get (Variables|Default|SetPlayerHealth (Math|Float|Clamp(Float) (- (Variables|Default|GetPlayerHealth) Damage) 0.0 1e+02)))
      (Variables|Default|SetHealthPercent (/ _output_get 1e+02))
      (if (>= (Variables|Default|GetPlayerHealth) 25.0)
        (Variables|Default|SetHealthBarColour (Class|ColorWheelHelper|HextoLinearColor "00FF01FF"))
        (else
          (Variables|Default|SetHealthBarColour (Class|ColorWheelHelper|HextoLinearColor "FF0000FF"))))
      (CallFunction|CheckHealth (Variables|Default|GetPlayerHealth)))
    (:then_1
      ;[1 1 1] LookAtPlayerOnHit
      (bind _asdangle_bp (Utilities|Casting|CastToDangle_BP (Game|GetPlayerCharacter 0)))
      (Transformation|SetActorRotation (Math|Rotator|MakeRotator (.roll (Math|Rotator|FindLookatRotation (Transformation|GetActorLocation) (Transformation|GetActorLocation _asdangle_bp))) 0.0 (.yaw (Math|Rotator|FindLookatRotation (Transformation|GetActorLocation) (Transformation|GetActorLocation _asdangle_bp)))))
      (CallFunction|GotHit (Game|GetPlayerCharacter 0)))))